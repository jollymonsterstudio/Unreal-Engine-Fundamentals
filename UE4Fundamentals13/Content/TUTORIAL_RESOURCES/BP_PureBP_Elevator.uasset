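; Tutorial elevator actor, built in pure Blueprint, that moves a static mesh along a spline.
; A timeline curve maps to distance along the spline, setting location plus roll and yaw, leaving pitch at zero.
; It starts at the first point, optionally auto-plays, and can restart or reverse on finishing.
; Entering the box plays from the start unless already playing; leaving reverses it unless already reversing.
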(event `self.ReceiveBeginPlay`
  (`SceneComponent.K2_SetWorldLocation` (`self.StaticMesh`) (`SplineComponent.GetLocationAtSplinePoint` (`self.Spline`) 0 "World") false false)
  (if (`self.AutoPlay`)
    (bind (_direction _movementcurve) (`Timeline|MovementTimeline` :!via `PlayFromStart` :!label _label)
      (:`Update`
        (`self.ProcessMovementTimeline` _movementcurve))
      (:`Finished`
        (`self.OnEndMovementTimeline`)))
    (`TimelineComponent.SetTimelineLengthMode` (`self.MovementTimeline`) "TL_LastKeyFrame")
    (else
      (goto _label :!via `Stop`))))

(event `self.Box.OnComponentBeginOverlap`
  (params (OverlappedComponent :type "PrimitiveComponent Object Reference") (OtherActor :type "Actor Object Reference") (OtherComp :type "PrimitiveComponent Object Reference") (OtherBodyIndex :type Integer) (bFromSweep :type Boolean) (SweepResult :type "HitResult Structure (by ref)"))
  (bind _movementtimeline (`self.MovementTimeline`))
  (if (not (`TimelineComponent.IsPlaying` _movementtimeline))
    (`TimelineComponent.PlayFromStart` _movementtimeline)))

(event `self.Box.OnComponentEndOverlap`
  (params (OverlappedComponent :type "PrimitiveComponent Object Reference") (OtherActor :type "Actor Object Reference") (OtherComp :type "PrimitiveComponent Object Reference") (OtherBodyIndex :type Integer))
  (bind _movementtimeline (`self.MovementTimeline`))
  (if (not (`TimelineComponent.IsReversing` _movementtimeline))
    (`TimelineComponent.Reverse` _movementtimeline)))

(fn `OnEndMovementTimeline`
  (if (`self.RestartOnEndTimeline`)
    (`TimelineComponent.PlayFromStart` (`self.MovementTimeline`))
    (elif (`self.ReverseOnEndTimeline`)
      (`TimelineComponent.Reverse` (`self.MovementTimeline`)))))

(fn `ProcessMovementTimeline`
  (params (Value :type "Float (double-precision)"))
  (bind _spline (`self.Spline`))
  (bind _returnvalue (* Value (`SplineComponent.GetSplineLength` _spline)))
  (bind (_returnvalue_roll _returnvalue_pitch _returnvalue_yaw) (`KismetMathLibrary.BreakRotator` (`SplineComponent.GetRotationAtDistanceAlongSpline` _spline _returnvalue "World")))
  (`SceneComponent.K2_SetWorldLocationAndRotation` (`self.StaticMesh`) (`SplineComponent.GetLocationAtDistanceAlongSpline` _spline _returnvalue "World") (`KismetMathLibrary.MakeRotator` _returnvalue_roll 0.0 _returnvalue_yaw) false false))

(fn `UserConstructionScript`)